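; JonneBP is a skeletal-mesh actor that pushes whatever component it hits.
; On each mesh hit it applies a scaled-down share of the normal impulse to the other component.
; The cooldown check after the push leads nowhere, as the Jonne voice sound and its timer-reset cooldown are disconnected.
; A node that disables physics simulation below a bone is also unwired, and PhysicalAnimation is unused.
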(event OnComponentHit(SkeletalMesh)
  (params (HitComponent :type Primitive%20Component%20Object%20Reference) (OtherActor :type Actor%20Object%20Reference) (OtherComp :type Primitive%20Component%20Object%20Reference) (NormalImpulse :type Vector :default "0, 0, 0") (Hit :type Hit%20Result%20Structure%20%28by%20ref%29))
  (Physics|AddImpulse OtherComp (* NormalImpulse 0.1) "None" false)
  (if (Variables|Default|GetIsOnCooldown)
    _))

(event Custom|CustomEvent_0
  (Variables|Default|SetIsOnCooldown false))

(fn ConstructionScript)